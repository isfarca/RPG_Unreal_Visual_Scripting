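; IntelligentDoors is a door actor that swings open while the player holds E and swings back on release.
; Box overlap begin and end both toggle the DoorManagerTextRender text and enable input for player 0, so input is never disabled.
; The RotationAnimation timeline drives SMDoor's relative yaw, zeroing world rotation before each update.
; The construction script sets the door's initial yaw from RotationOfDoor.
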(event `self.Box.OnComponentBeginOverlap`
  (params (OverlappedComponent :type "PrimitiveComponent Object Reference") (OtherActor :type "Actor Object Reference") (OtherComp :type "PrimitiveComponent Object Reference") (OtherBodyIndex :type Integer) (bFromSweep :type Boolean) (SweepResult :type "HitResult Structure (by ref)"))
  ;[1 1 1] Enable input
  (`SceneComponent.ToggleVisibility` (`self.DoorManagerTextRender`) false :!label _label)
  (`self.EnableInput` (`GameplayStatics.GetPlayerController` 0)))

(event `self.Box.OnComponentEndOverlap`
  (params (OverlappedComponent :type "PrimitiveComponent Object Reference") (OtherActor :type "Actor Object Reference") (OtherComp :type "PrimitiveComponent Object Reference") (OtherBodyIndex :type Integer))
  ;[1 1 1] Enable input
  (goto _label))

(event `Key|E`
  (params (Key :type "Key Structure"))
  (:`Pressed`
    ;[1 1 1] Door animation
    (bind (_direction _newtrack_0) (`Timeline|RotationAnimation` :!label _label_2)
      (:`Update`
        (`SceneComponent.K2_SetWorldRotation` :`self` (`self.SM_Door`))
        (`SceneComponent.K2_SetRelativeRotation` (`self.SM_Door`) (`KismetMathLibrary.MakeRotator` 0.0 0.0 _newtrack_0) false false))))
  (:`Released`
    (goto _label_2 :!via `Reverse`)))

(fn `UserConstructionScript`
  (`SceneComponent.K2_SetRelativeRotation` (`self.SM_Door`) (`KismetMathLibrary.MakeRotator` 0.0 0.0 (`self.RotationOfDoor`)) false false))